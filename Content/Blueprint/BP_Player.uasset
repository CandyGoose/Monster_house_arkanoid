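; Player pawn for a ball game: moves sideways along world Y with swept offsets and manages lives and pausing.
; Spawns BP_Ball at a spawn point and binds its death event, which costs one HP and respawns a ball.
; At zero HP it shows the BadG widget, then opens MainMenu after a delay or on Space.
; Escape opens a cached PauseMenu in UI-only input mode and pauses the game, unless the game is over.
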(event `self.ReceiveBeginPlay`
  (`self.Spawn_Ball`)
  (set `self.KeyEnabled` true))

(event `InputAxis|MoveRight`
  (params (AxisValue :type "Float (single-precision)"))
  (`self.K2_AddActorWorldOffset` (`KismetMathLibrary.MakeVector` 0.0 (* AxisValue (`self.Speed`) (`GameplayStatics.GetWorldDeltaSeconds`))) true))

(event `Spawn_Ball`
  (bind _spawnpointball (`self.SpawnPointBall`))
  (bind _returnvalue (`|SpawnActorFromClass` "/Game/Blueprint/BP_Ball.BP_Ball_C" (`KismetMathLibrary.MakeTransform` (`SceneComponent.K2_GetComponentLocation` _spawnpointball) (`SceneComponent.K2_GetComponentRotation` _spawnpointball)) "Undefined" "OverrideRootScale" null null))
  (add `/Game/Blueprint/BP_Ball.Death` _returnvalue (delegate `OnDeath_Event`)))

(event `OnDeath_Event`
  (set `self.HP` (- (`self.HP`) 1))
  (if (<= (`self.HP`) 0)
    (set `self.KeyEnabled` false)
    (bind _returnvalue (`|CreateWidget` "/Game/UI/BadG.BadG_C"))
    (`UserWidget.AddToViewport` _returnvalue 0)
    (`KismetSystemLibrary.Delay` 16.0)
    (`Widget.RemoveFromParent` _returnvalue :!label _label)
    (`GameplayStatics.OpenLevel` "MainMenu")
    (else
      (`self.Spawn_Ball`))))

(event `Key|SpaceBar`
  (params (Key :type "Key Structure"))
  (:`Pressed`
    (if (<= (`self.HP`) 0)
      (goto _label))))

(event `Key|Escape` :paused true
  (params (Key :type "Key Structure"))
  (bind _returnvalue (`GameplayStatics.GetPlayerController` 0))
  (bind _pause (`self.Pause`))
  (:`Pressed`
    (if (`self.KeyEnabled`)
      (`/Engine/EditorBlueprintResources/StandardMacros.IsValid` (`self.Pause`)
        (:`Is Valid`
          _)
        (:`Is Not Valid`
          (bind _returnvalue_2 (`|CreateWidget` "/Game/UI/PauseMenu.PauseMenu_C"))
          (set `self.Pause` _returnvalue_2)))
      (set `PlayerController.bShowMouseCursor` true _returnvalue)
      (`WidgetBlueprintLibrary.SetInputMode_UIOnlyEx` _returnvalue _pause)
      (`UserWidget.AddToViewport` _pause 0)
      (`GameplayStatics.SetGamePaused` true))))

(fn `UserConstructionScript`)