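; BP_Ball is a self-moving ball that bounces off blocking surfaces and dies on entering a KillZVolume.
; Each Tick it sweeps along Direction at Speed, reflects off the hit normal with Z zeroed, and slightly increases Speed per bounce.
; The first bounce also creates the HUD widget through a DoOnce.
; Overlapping a KillZVolume triggers CallDeath and destroys the actor.
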(event `self.ReceiveBeginPlay`)

(event `self.ReceiveActorBeginOverlap`
  (params (OtherActor :type "Actor Object Reference"))
  (cast `KillZVolume` OtherActor)
  (`self.Death`)
  (`self.K2_DestroyActor`))

(event `self.ReceiveTick`
  (params (DeltaSeconds :type "Float (single-precision)"))
  (bind _sweephitresult (`self.K2_AddActorWorldOffset` (* (* (`self.Direction`) (`self.Speed`)) DeltaSeconds) true))
  (bind (_bblockinghit _binitialoverlap _time _distance _location _impactpoint _normal) (`GameplayStatics.BreakHitResult` _sweephitresult))
  (if _bblockinghit
    (bind (_returnvalue_x _returnvalue_y) (`KismetMathLibrary.BreakVector` (`KismetMathLibrary.GetReflectionVector` (`self.Direction`) _normal)))
    (set `self.Direction` (`KismetMathLibrary.MakeVector` _returnvalue_x _returnvalue_y))
    (set `self.Speed` (+ (`self.Speed`) 0.1))
    (`/Engine/EditorBlueprintResources/StandardMacros.DoOnce` false
      (:`Completed`
        (bind _returnvalue (`|CreateWidget` "/Game/UI/HUD.HUD_C"))
        (`UserWidget.AddToViewport` _returnvalue 0)))))

(fn `UserConstructionScript`)