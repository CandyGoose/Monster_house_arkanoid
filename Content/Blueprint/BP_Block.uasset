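; BP_Block is a breakable block that loses HP and plays a hit sound when struck by BP_Ball.
; Surviving hits show a cracked material and randomly trigger either a point-light flicker, looped through DoN and Delay, or one of three extra sounds.
; At zero HP it removes its cube, then destroys itself after a delay and shows the GoodG widget if no blocks remain.
; Space removes that widget and opens MainMenu.
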(event `self.ReceiveBeginPlay`
  (`SceneComponent.ToggleVisibility` (`self.PointLight`) false)
  (`ActorComponent.ToggleActive` (`self.Audio`))
  (`ActorComponent.ToggleActive` (`self.Audio1`))
  (`ActorComponent.ToggleActive` (`self.Audio2`))
  (`ActorComponent.ToggleActive` (`self.Hit`)))

(event `self.Cube.OnComponentHit`
  (params (HitComponent :type "PrimitiveComponent Object Reference") (OtherActor :type "Actor Object Reference") (OtherComp :type "PrimitiveComponent Object Reference") (NormalImpulse :type "Vector Structure") (Hit :type "HitResult Structure (by ref)"))
  (bind _hit (`self.Hit`))
  (bind _event (`self.Event`))
  (bind _audio (`self.Audio`))
  (bind _event_2 (`self.Event`))
  (bind _audio1 (`self.Audio1`))
  (bind _audio2 (`self.Audio2`))
  (cast `/Game/Blueprint/BP_Ball` OtherActor)
  (`ActorComponent.SetActive` _hit true false)
  (`AudioComponent.Play` _hit 0.0)
  (set `self.Event` (`KismetMathLibrary.RandomIntegerInRange` 0 7))
  ;[1 1 1] HP
  (bind _result (`/Engine/EditorBlueprintResources/StandardMacros.DecrementInt` (`self.HP`))
    (:`  `
      (if (> _result 0)
        (`PrimitiveComponent.SetMaterial` (`self.Cube`) 0 "/Game/Environment/Materials/Box_cracked.Box_cracked")
        (if (== _event 0)
          (`/Engine/EditorBlueprintResources/StandardMacros.Do N` 20 :!label _label
            (:`Exit`
              (`SceneComponent.ToggleVisibility` (`self.PointLight`) false)
              (`KismetSystemLibrary.Delay` 0.05)
              (goto _label)))
          (elif (== _event 1)
            (set `self.Event` (`KismetMathLibrary.RandomIntegerInRange` 0 2))
            (if (== _event_2 0)
              (`ActorComponent.ToggleActive` _audio)
              (`AudioComponent.Play` _audio 0.0)
              (elif (== _event_2 1)
                (`ActorComponent.ToggleActive` _audio1)
                (`AudioComponent.Play` _audio1 0.0)
                (else
                  (`ActorComponent.ToggleActive` _audio2)
                  (`AudioComponent.Play` _audio2 0.0))))))
        (else
          (`ActorComponent.K2_DestroyComponent` (`self.Cube`))
          (`KismetSystemLibrary.Delay` 1.0)
          (`self.K2_DestroyActor`)
          (bind _outactors (`GameplayStatics.GetAllActorsOfClass` "BP_Block_C"))
          (if (not (> (`KismetArrayLibrary.Array_Length` _outactors) 0))
            (bind _returnvalue (`|CreateWidget` "/Game/UI/GoodG.GoodG_C"))
            (`UserWidget.AddToViewport` _returnvalue 5000)))))))

(event `Key|SpaceBar`
  (params (Key :type "Key Structure"))
  (:`Pressed`
    (`Widget.RemoveFromParent` (stale `self.Cube.OnComponentHit` _returnvalue))
    (`GameplayStatics.OpenLevel` "MainMenu")))

(fn `UserConstructionScript`)